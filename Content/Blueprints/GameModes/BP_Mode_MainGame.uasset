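; Main game mode for the photo game that owns saving and loading of player progress.
; On BeginPlay it loads the save slot into the player character, or creates an empty save file if none exists.
; A SaveGame event copies taken photos, inventory, equipped camo and transform from the player into the BP_SaveData_PhotoGame object and writes it back to the slot.
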(event Custom|Save%20Game
  (bind _returnvalue (SaveGame|LoadGamefromSlot (Variables|Default|GetSave%20Slot%20Name)))
  (bind _asbp_save_data_photo_game (Utilities|Casting|CastToBP_SaveData_PhotoGame _returnvalue))
  (bind _asbp_player_char (Utilities|Casting|CastToBP_PlayerChar (Game|Player|GetPlayerPawn 0)))
  (Variables|/Game/Blueprints/BP_SaveData_PhotoGame.BP_SaveData_PhotoGame_C|SetPhoto%20Data _asbp_save_data_photo_game (Variables|/Game/Blueprints/BP_PlayerChar.BP_PlayerChar_C|GetTaken%20Photos _asbp_player_char))
  (Variables|/Game/Blueprints/BP_SaveData_PhotoGame.BP_SaveData_PhotoGame_C|SetPlayer%20Inventory _asbp_save_data_photo_game (Variables|/Game/Blueprints/BP_PlayerChar.BP_PlayerChar_C|GetInventory _asbp_player_char))
  (Variables|/Game/Blueprints/BP_SaveData_PhotoGame.BP_SaveData_PhotoGame_C|SetPlayer%20Camo _asbp_save_data_photo_game (Variables|/Game/Blueprints/BP_PlayerChar.BP_PlayerChar_C|GetEquipped%20Camo _asbp_player_char))
  (Variables|/Game/Blueprints/BP_SaveData_PhotoGame.BP_SaveData_PhotoGame_C|SetPlayer%20Transform _asbp_save_data_photo_game (Transformation|GetActorTransform _asbp_player_char))
  (SaveGame|SaveGametoSlot _asbp_save_data_photo_game (Variables|Default|GetSave%20Slot%20Name)))

(event EventBeginPlay
  (bind _returnvalue (SaveGame|DoesSaveGameExist (Variables|Default|GetSave%20Slot%20Name)))
  (if _returnvalue
    (|LoadGameonGameStart)
    (else
      (|CreateSaveFile))))

(event EventTick
  (params (DeltaSeconds :type Float%20%28single-precision%29)))

(fn ConstructionScript)