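; BP_Harvest_Berry is a harvestable berry actor that shrinks as it takes damage and is destroyed when its health runs out.
; BeginPlay records the starting scale after calling the parent.
; AnyDamage subtracts damage from Health, then either destroys the actor or scales it by Health over a fixed 100 and calls DropToGround.
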(event EventBeginPlay
  (|CallParentFunction)
  (Variables|Default|SetStarting%20Scale (Transformation|GetActorScale3D)))

(event Collision|EventActorBeginOverlap
  (params (OtherActor :type Actor%20Object%20Reference))
  (|CallParentFunction OtherActor) ; This node is disabled and will not be called.\nDrag off pins to build functionality.
)

(event EventTick
  (params (DeltaSeconds :type Float%20%28single-precision%29))
  (|CallParentFunction DeltaSeconds) ; This node is disabled and will not be called.\nDrag off pins to build functionality.
)

(event Game|Damage|EventAnyDamage
  (params (Damage :type Float%20%28single-precision%29) (DamageType :type Damage%20Type%20Object%20Reference) (InstigatedBy :type Controller%20Object%20Reference) (DamageCauser :type Actor%20Object%20Reference))
  (bind _output_get (Variables|Default|SetHealth (- (Variables|Default|GetHealth) Damage)))
  (if (<= _output_get 0.0)
    (Actor|DestroyActor)
    (else
      (Transformation|SetActorScale3D (* (Variables|Default|GetStarting%20Scale) (/ (Variables|Default|GetHealth) 1e+02)))
      (CallFunction|DroptoGround))))

(fn ConstructionScript
  (|CallParentFunction))