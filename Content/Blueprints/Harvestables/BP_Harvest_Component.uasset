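; Actor component that makes its owner a harvestable pickup, granting a set item and amount to the player's inventory.
; Harvest looks the item up in the player's inventory map, adding to the existing count or inserting a new entry.
; New items also get a button in the player's pause menu.
; The owning actor is destroyed after every harvest.
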(event EventBeginPlay)

(event EventTick
  (params (DeltaSeconds :type Float%20%28single-precision%29)))

(fn Harvest
  (params (Player :type BP%20Player%20Char%20Object%20Reference))
  (bind _data_to_give_to_player (Variables|Default|GetData%20to%20Give%20to%20Player))
  (bind _inventory (Variables|/Game/Blueprints/BP_PlayerChar.BP_PlayerChar_C|GetInventory Player))
  (bind (_value _returnvalue) (Utilities|Map|Find _inventory _data_to_give_to_player))
  (if _returnvalue
    (|IncreaseInventoryAmount _inventory _value)
    (else
      (|AddNewInventoryItem _inventory)
      (Default|AddInventoryButton (Variables|/Game/Blueprints/BP_PlayerChar.BP_PlayerChar_C|GetPause%20Menu Player) (Variables|Default|GetData%20to%20Give%20to%20Player))))
  (|DestroySelf)
  (return))