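; BP_Harvestable is an actor for a harvestable world object.
; Its Harvest function passes the Player straight to BPHarvestComponent, which handles the harvest.
; On BeginPlay it snaps to the ground with a short downward Visibility trace, lifting itself by the scaled capsule half-height without checking whether the trace hit.
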(event EventBeginPlay
  (CallFunction|DroptoGround))

(event Collision|EventActorBeginOverlap
  (params (OtherActor :type Actor%20Object%20Reference)))

(event EventTick
  (params (DeltaSeconds :type Float%20%28single-precision%29)))

(fn ConstructionScript)

(fn Harvest
  (params (Player :type BP%20Player%20Char%20Object%20Reference))
  (Default|Harvest (Variables|Default|GetBP_Harvest_Component) Player))

(fn DroptoGround
  (bind _returnvalue (Transformation|GetActorLocation))
  (bind _outhit (Collision|LineTraceByChannel _returnvalue (+ _returnvalue (* (Math|Vector|VectorUp) -512.0)) "TraceTypeQuery1" false 0 "None"))
  (Transformation|SetActorLocation (+ (.ImpactPoint (Collision|BreakHitResult _outhit)) (Math|Vector|MakeVector 0.0 0.0 (* (Variables|/Script/Engine.CapsuleComponent|GetCapsuleHalfHeight (Variables|Default|GetCollider)) (.z (Transformation|GetActorScale3D))))) false false))