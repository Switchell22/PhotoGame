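; First-person player character for a stealth photography game, handling movement, HUD, pause/crafting menu and a hold-to-view photo album.
; Photos trace for a PhotoAI subject, score its facing against the camera, record and export the render-target capture, then the game saves.
; Stealth percentage combines crouching, stillness, equipped camo on the traced surface and external bonuses.
; Interact line-traces to harvest objects or place the equipped item.
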(event OnSeePawn(PawnSensing)
  (params (Pawn :type Pawn%20Object%20Reference))
  (Utilities|Casting|CastToBP_Parent_PhotoAI Pawn)
  (Development|PrintString "AI Visible" true true "(R=0.000000,G=0.660000,B=1.000000,A=1.000000)" 2.0 "Is AI Seen by Player?"))

(event EventBeginPlay
  (bind _returnvalue (UserInterface|CreateWidget "/Game/UI/Menus/W_PlayerHUD.W_PlayerHUD_C"))
  (bind _output_get (Variables|UI|SetGame%20HUD _returnvalue))
  (bind _returnvalue_2 (UserInterface|CreateWidget "/Game/UI/Menus/W_CraftingMenu.W_CraftingMenu_C"))
  (Variables|UI|SetPause%20Menu _returnvalue_2)
  (UserInterface|Viewport|AddtoViewport _output_get 0)
  (Collision|SetCollisionProfileName (Variables|Collision|GetCapsuleComponent) "player" true :!class /Script/Engine.PrimitiveComponent)
  (bind _returnvalue_3 (UserInterface|CreateWidget "/Game/UI/Menus/W_PhotoAlbum.W_PhotoAlbum_C"))
  (Variables|UI|SetPhoto%20Album _returnvalue_3))

(event Collision|EventActorBeginOverlap
  (params (OtherActor :type Actor%20Object%20Reference)))

(event EventTick
  (params (DeltaSeconds :type Float%20%28single-precision%29))
  (Class|PawnMovementComponent|ConsumeInputVector (Variables|Character|GetCharacterMovement)))

(event Input|ActionEvents|InputActionInput_Pause
  (params (Key :type Key%20Structure :default "None"))
  (bind _returnvalue (Game|GetPlayerController 0))
  (bind _game_hud (Variables|UI|GetGame%20HUD))
  (bind _pause_menu (Variables|UI|GetPause%20Menu))
  (:Pressed
    (if (Game|IsGamePaused)
      (Game|SetGamePaused false)
      (Development|PrintString "Game Unpaused")
      (Variables|/Script/Engine.PlayerController|SetbShowMouseCursor _returnvalue false)
      (UserInterface|Viewport|AddtoViewport _game_hud 0)
      (Widget|RemovefromParent _pause_menu)
      (else
        (Game|SetGamePaused true)
        (Development|PrintString "Game Paused")
        (Variables|/Script/Engine.PlayerController|SetbShowMouseCursor _returnvalue true)
        (Widget|RemovefromParent _game_hud)
        (UserInterface|Viewport|AddtoViewport _pause_menu 0)))))

(event Input|ActionEvents|InputActionInput_TakePhoto
  (params (Key :type Key%20Structure :default "None"))
  (:Pressed
    (CallFunction|TakePhoto)
    (bind _asbp_mode_main_game (Utilities|Casting|CastToBP_Mode_MainGame (Game|GetGameMode)))
    (Default|SaveGame _asbp_mode_main_game)))

(event Input|ActionEvents|InputActionInput_Interact
  (params (Key :type Key%20Structure :default "None"))
  (:Pressed
    (if (== (Variables|Gameplay|GetEquipped%20Item) 0)
      (CallFunction|PickUpObject)
      (else
        (CallFunction|PlaceObject)))))

(event Input|ActionEvents|InputActionInput_Crouch
  (params (Key :type Key%20Structure :default "None"))
  (bind _camera (Variables|Default|GetCamera))
  (:Pressed
    (Character|Crouch)
    (Transformation|SetRelativeLocation _camera "0, 0,32.000000" false false))
  (:Released
    (Character|UnCrouch)
    (Transformation|SetRelativeLocation _camera "0, 0,64.000000" false false)))

(event Input|ActionEvents|InputActionInput_PhotoAlbum
  (params (Key :type Key%20Structure :default "None"))
  (bind _returnvalue (Game|GetPlayerController 0))
  (bind _photo_album (Variables|UI|GetPhoto%20Album))
  (:Pressed
    (UserInterface|Viewport|AddtoViewport _photo_album 0)
    (Variables|/Script/Engine.PlayerController|SetbShowMouseCursor _returnvalue true)
    (Game|SetGamePaused true))
  (:Released
    (Widget|RemovefromParent _photo_album)
    (Variables|/Script/Engine.PlayerController|SetbShowMouseCursor _returnvalue false)
    (Game|SetGamePaused false)))

(event Input|AxisEvents|InputAxisAxis_Camera_Up
  (params (AxisValue :type Float%20%28single-precision%29))
  (Pawn|Input|AddControllerPitchInput (* AxisValue -1.0)))

(event Input|AxisEvents|InputAxisAxis_Camera_Right
  (params (AxisValue :type Float%20%28single-precision%29))
  (Pawn|Input|AddControllerYawInput AxisValue))

(event Input|AxisEvents|InputAxisAxis_Move_Forward
  (params (AxisValue :type Float%20%28single-precision%29))
  (Class|PawnMovementComponent|AddInputVector (Variables|Character|GetCharacterMovement) (* AxisValue (Math|Vector|GetForwardVector (Variables|Default|GetCamera))) false))

(event Input|AxisEvents|InputAxisAxis_Move_Right
  (params (AxisValue :type Float%20%28single-precision%29))
  (Class|PawnMovementComponent|AddInputVector (Variables|Character|GetCharacterMovement) (* AxisValue (Math|Vector|GetRightVector (Variables|Default|GetCamera))) false))

(fn ConstructionScript)

(fn GetStealthPercentage
  (return (Math|Float|Clamp(Float) (+ (|StealthBonusfromCrouching) (CallFunction|GetCamoBonusfromSurface) (|StealthBonusfromStayingStill) (Variables|Gameplay|GetStealth%20Given%20by%20Other%20Objects)) 0.0 1e+02)))

(fn GetCamoBonusfromSurface
  (return (.Value (Utilities|Map|Find (.surfacestealth (Variables|Gameplay|GetEquipped%20Camo)) (CallFunction|GetSurfaceTypeStandingon)))))

(fn GetSurfaceTypeStandingon
  (bind _returnvalue (Transformation|GetActorLocation))
  (bind _outhit (Collision|LineTraceByChannel _returnvalue (- _returnvalue "0,0,2300.000000") "TraceTypeQuery2" false 0 "ForDuration"))
  (return (Collision|GetSurfaceType _outhit)))

(fn PickUpObject
  (bind _returnvalue (Transformation|GetActorLocation))
  (bind _outhit (Collision|LineTraceByChannel _returnvalue (+ _returnvalue (* (Math|Vector|GetForwardVector (Variables|Default|GetCamera)) 256.0)) "TraceTypeQuery2" false 0 "ForDuration" true "(R=0.122074,G=0.000000,B=1.000000,A=1.000000)"))
  (bind _asbp_harvestable (Utilities|Casting|CastToBP_Harvestable (.HitActor (Collision|BreakHitResult _outhit))))
  (Default|Harvest _asbp_harvestable self))

(fn PlaceObject
  (bind _returnvalue (Transformation|GetActorLocation))
  (bind (_outhit _returnvalue_2) (Collision|LineTraceByChannel _returnvalue (+ _returnvalue (* (Math|Vector|GetForwardVector (Variables|Default|GetCamera)) 512.0)) "TraceTypeQuery2" false 0 "None"))
  (if _returnvalue_2
    (Game|SpawnActorfromClass (Variables|Gameplay|GetEquipped%20Item) (Math|Transform|MakeTransform (+ (.ImpactPoint (Collision|BreakHitResult _outhit)) "0,0,64.000000") (Transformation|GetActorRotation) "1.000000,1.000000,1.000000") "AdjustIfPossibleButAlwaysSpawn" 0 0)
    (Variables|Gameplay|SetEquipped%20Item 0)
    (Variables|UI|SetEquipped%20Item%20Icon 0)))

(fn TakePhoto
  (Audio|PlaySoundatLocation "/Game/Audio/SFX/Cue_Camera.Cue_Camera" "0, 0, 0" "0, 0, 0" 1.0 1.0 0.0 0 0 0 0)
  (Rendering|SceneCapture|CaptureScene (Variables|Default|GetSceneCaptureComponent2D) :!class /Script/Engine.SceneCaptureComponent2D)
  (bind _hitactor (|LineTrace))
  (bind _asbp_parent_photo_ai (Utilities|Casting|CastToBP_Parent_PhotoAI _hitactor))
  (bind _filename (|AddPhotoDatatoArray (|CalculateScore _asbp_parent_photo_ai) _asbp_parent_photo_ai))
  (Rendering|ExportRenderTarget (Variables|/Script/Engine.SceneCaptureComponent2D|GetTextureTarget (Variables|Default|GetSceneCaptureComponent2D)) (Variables|Default|GetPhoto%20File%20Path) _filename)
  (|PrintPhotoScore (|CalculateScore _asbp_parent_photo_ai)))