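; Parent AI for photographable creatures that eat harvestable berries, flee the player and leave footprint decals on a repeating delay.
; AI perception sends it toward seen berries; while one is focused, Tick raises Distraction and damages the berry when close.
; Pawn sensing triggers flight only if player stealth plus Distraction is below StealthThreshold, moving to a ground-traced point directly away from the player.
; An empty InteractWithDistraction event runs each Tick.
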(event OnSeePawn(PawnSensing)
  (params (Pawn :type Pawn%20Object%20Reference))
  (bind _asbp_player_char (Utilities|Casting|CastToBP_PlayerChar Pawn))
  (|RunfromPlayer _asbp_player_char))

(event OnTargetPerceptionUpdated(AIPerception)
  (params (Actor :type Actor%20Object%20Reference) (Stimulus :type AI%20Stimulus%20Structure))
  (bind _asbp_harvest_berry (Utilities|Casting|CastToBP_Harvest_Berry Actor))
  (Development|PrintString "I saw a berry!" true true "(R=0.000000,G=0.660000,B=1.000000,A=1.000000)" 2.0 "BerrySeen")
  (AI|AIMoveTo self (Transformation|GetActorLocation _asbp_harvest_berry) _asbp_harvest_berry 16.0 true
    (:then
      (Variables|Default|SetItem%20to%20Focus _asbp_harvest_berry))
    (:OnFail
      (Variables|Default|SetItem%20to%20Focus 0))))

(event Custom|Interact%20with%20Distraction)

(event Custom|No%20Longer%20Distracted
  (Variables|Default|SetDistraction 0.0))

(event EventBeginPlay
  (Utilities|FlowControl|Delay 0.5 :!label _label)
  (CallFunction|SpawnFootprint)
  (goto _label))

(event Collision|EventActorBeginOverlap
  (params (OtherActor :type Actor%20Object%20Reference)))

(event EventTick
  (params (DeltaSeconds :type Float%20%28single-precision%29))
  (CallFunction|InteractwithDistraction)
  (CallFunction|UpdateifIAmDistracted DeltaSeconds))

(fn ConstructionScript)

(fn HidefromTarget
  (params (Actor%20to%20Hide%20From :type Pawn%20Object%20Reference))
  (bind _returnvalue (Transformation|GetActorLocation))
  (AI|Navigation|SimpleMovetoLocation (AI|GetAIController self) (+ (* (Math|Vector|GetUnitDirection(Vector) (Transformation|GetActorLocation Actor%20to%20Hide%20From) _returnvalue) 16.0) _returnvalue)))

(fn SpawnFootprint
  (CallFunction|SpawnFootprint self "/Game/Materials/M_Footprint.M_Footprint" "8.000000,64.000000,64.000000"))

(fn CanSeePlayer?
  (bind _asbp_player_char (Utilities|Casting|CastToBP_PlayerChar (Game|Player|GetPlayerPawn 0)))
  (Development|PrintString (Utilities|String|Append "Player Stealth: " (Utilities|String|ToString(Float) (Default|GetStealthPercentage _asbp_player_char)) "| Distraction: " (Utilities|String|ToString(Float) (Variables|Default|GetDistraction)) "| Total Stealth: " (Utilities|String|ToString(Float) (+ (Default|GetStealthPercentage _asbp_player_char) (Variables|Default|GetDistraction))) "| Can See Player? " (Utilities|String|ToString(Boolean) (< (+ (Default|GetStealthPercentage _asbp_player_char) (Variables|Default|GetDistraction)) (Variables|Default|GetStealth%20Threshold)))) true true "(R=1.000000,G=0.000000,B=0.207984,A=1.000000)" 2.0 "StealthThreshold")
  (return (< (+ (Default|GetStealthPercentage _asbp_player_char) (Variables|Default|GetDistraction)) (Variables|Default|GetStealth%20Threshold))))

(fn UpdateifIAmDistracted
  (params (Delta%20Seconds :type Float%20%28double-precision%29))
  (bind _returnvalue (Transformation|GetActorLocation))
  (bind _item_to_focus (Variables|Default|GetItem%20to%20Focus))
  (bind _returnvalue_2 (Transformation|GetActorLocation _item_to_focus))
  (bind _returnvalue_3 (Math|Vector|Distance(Vector) _returnvalue _returnvalue_2))
  (if (Utilities|IsValid (Variables|Default|GetItem%20to%20Focus)) ; Does distraction exist?
    (Development|PrintString (Utilities|String|Append "Distance to disctraction: " (Utilities|String|ToString(Float) _returnvalue_3)) true true "(R=0.000000,G=0.660000,B=1.000000,A=1.000000)" 2.0 "DistanceToDistraction")
    (if (<= _returnvalue_3 192.0) ; Am I close enough to distraction?
      (Development|PrintString "I'm eating this berry!" true true "(R=0.000000,G=0.660000,B=1.000000,A=1.000000)" 2.0 "Eating?")
      (Game|Damage|ApplyDamage (Variables|Default|GetItem%20to%20Focus) (* Delta%20Seconds 2e+01) 0 0)
      (else
        (Development|PrintString "I'm chasing the berry, but not eating it!" true true "(R=0.000000,G=0.660000,B=1.000000,A=1.000000)" 2.0 "Eating?")))
    (Variables|Default|SetDistraction 25.0)
    (else
      (Variables|Default|SetDistraction 0.0)))
  (return))